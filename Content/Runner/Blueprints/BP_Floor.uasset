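; Floor tile for a runner game that asks BP_RunnerGM to extend the floor when its box is overlapped and exposes an arrow-based attach point.
; Its construction script builds lane spawn points, shuffles them and fills a few with child-actor obstacles through a chain of separately rolled chance checks.
; Moving obstacles are throttled by a game-mode floor counter, which resets when one spawns.
; The player speed-up logic is disconnected.
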(event `self.Box.OnComponentBeginOverlap`
  (params (OverlappedComponent :type "PrimitiveComponent Object Reference") (OtherActor :type "Actor Object Reference") (OtherComp :type "PrimitiveComponent Object Reference") (OtherBodyIndex :type Integer) (bFromSweep :type Boolean) (SweepResult :type "HitResult Structure (by ref)"))
  ;[1 1 1] Extend Floor
  (bind _asbp_runner_gm (cast `/Game/Runner/Blueprints/BP_RunnerGM` (`GameplayStatics.GetGameMode`)))
  (`/Game/Runner/Blueprints/BP_RunnerGM.ExtendFloor` _asbp_runner_gm))

(fn `Get AttachPoint`
  (returns (ReturnValue :type "Transform Structure"))
  (return (`SceneComponent.K2_GetComponentToWorld` (`self.Arrow`))))

(fn `Setup Spawn Spoints`
  (for _array_element (`self.Lane Position`)
    (for _index (range 2)
      (bind _returnvalue (`AddComponent|NODE_AddArrowComponent-0` :`RelativeTransform` (`KismetMathLibrary.MakeTransform` (`KismetMathLibrary.MakeVector` (* _index 650.0) _array_element))))
      (`KismetArrayLibrary.Array_Add` (`self.SpawnPoints`) (`SceneComponent.K2_GetComponentToWorld` _returnvalue)))))

(fn `Spawn Moving Obstacles`
  (params (Selection :type Integer) (RelativeTransform :type "Transform Structure"))
  (bind _asbp_runner_gm (cast `/Game/Runner/Blueprints/BP_RunnerGM` (`GameplayStatics.GetGameMode`)))
  (if (> (`/Game/Runner/Blueprints/BP_RunnerGM.Floor count for obstacles` _asbp_runner_gm) (`KismetMathLibrary.RandomIntegerInRange` 10 20))
    (switch `int` Selection
      (:`0`
        (`AddComponent|NODE_AddChildActorComponent-5` :`RelativeTransform` RelativeTransform))
      (:`1`
        (`AddComponent|NODE_AddChildActorComponent-6` :`RelativeTransform` RelativeTransform)))
    (set `/Game/Runner/Blueprints/BP_RunnerGM.Floor count for obstacles` 0 _asbp_runner_gm)))

(fn `Spawn Obstacles`
  (bind _returnvalue (`KismetMathLibrary.RandomIntegerInRange` 0 100))
  (bind _output_get (set `self.Random Spawn Points` (`self.SpawnPoints`)))
  (`KismetArrayLibrary.Array_Shuffle` _output_get)
  (for _index (range (+ (`KismetMathLibrary.RandomIntegerInRange` 0 2) 1))
    ;[0.008548 0 1] Ajouter obstacles
    ;;[1 0.7702 0.03871] Random Obstactles
    (if (`KismetMathLibrary.InRange_IntInt` _returnvalue)
      (bind _returnvalue_2 (`KismetMathLibrary.MakeRelativeTransform` (`|GetArrayItem` (`self.Random Spawn Points`) _index) (`self.GetTransform`)))
      (`AddComponent|NODE_AddChildActorComponent-1` :`RelativeTransform` _returnvalue_2)
      (elif (`KismetMathLibrary.InRange_IntInt` _returnvalue 11 20)
        (`AddComponent|NODE_AddChildActorComponent-2` :`RelativeTransform` _returnvalue_2)
        (elif (`KismetMathLibrary.InRange_IntInt` _returnvalue 21 30)
          (`AddComponent|NODE_AddChildActorComponent-3` :`RelativeTransform` _returnvalue_2)
          (elif (`KismetMathLibrary.InRange_IntInt` _returnvalue 31 40)
            (`AddComponent|NODE_AddChildActorComponent-4` :`RelativeTransform` _returnvalue_2)
            (elif (`KismetMathLibrary.InRange_IntInt` _returnvalue 41 50)
              (`AddComponent|NODE_AddChildActorComponent-8` :`RelativeTransform` _returnvalue_2)
              (elif (`KismetMathLibrary.InRange_IntInt` _returnvalue 51 60)
                (`AddComponent|NODE_AddChildActorComponent-9` :`RelativeTransform` _returnvalue_2)
                (elif (`KismetMathLibrary.InRange_IntInt` _returnvalue 61 70)
                  (`self.Spawn Moving Obstacles` 0 _returnvalue_2)
                  (elif (`KismetMathLibrary.InRange_IntInt` _returnvalue 71 80)
                    (`AddComponent|NODE_AddChildActorComponent-10` :`RelativeTransform` _returnvalue_2)
                    (elif (`KismetMathLibrary.InRange_IntInt` _returnvalue 81 100)
                      (`AddComponent|NODE_AddChildActorComponent-11` :`RelativeTransform` _returnvalue_2))))))))))))

(fn `UserConstructionScript`
  (`self.Setup Spawn Spoints`)
  (`self.Spawn Obstacles`))
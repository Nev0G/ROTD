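; BP_Obstacles_Points is a coin-style score pickup for the runner game.
; When BP_Runner overlaps it, it adds one to the runner's Score, plays the Coin sound in 2D and destroys itself.
; It then finds the runner again via GetActorOfClass and calls HighscoreCalculate on it to update the highscore.
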(event `self.ReceiveActorBeginOverlap`
  (params (OtherActor :type "Actor Object Reference"))
  (bind _asbp_runner (cast `/Game/Runner/Blueprints/BP_Runner` OtherActor))
  (set `/Game/Runner/Blueprints/BP_Runner.Score` (+ 1 (`/Game/Runner/Blueprints/BP_Runner.Score` _asbp_runner)) _asbp_runner)
  (`GameplayStatics.PlaySound2D` "/Game/Runner/Sounds/Effects/coin.coin" 1.0 1.0 0.0 null null)
  (`self.K2_DestroyActor`)
  (bind _returnvalue (`GameplayStatics.GetActorOfClass` "/Game/Runner/Blueprints/BP_Runner.BP_Runner_C"))
  (`/Game/Runner/Blueprints/BP_Runner.HighscoreCalculate` _returnvalue))

(fn `UserConstructionScript`
  (`parent.UserConstructionScript`))
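; BP_Turret is a runner obstacle that spots the player's BP_Runner and shoots at it.
; When PawnSensing sees the runner, it snaps its rotation toward it and, after a short delay, spawns BP_Bullets from its Arrow component.
; Overlapping the runner costs it health, refreshes the on-screen health text, shakes the camera and explodes the turret.
; Damage, noted as coming from the shotgun, drains its Health until it explodes.
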(event `self.ReceiveActorBeginOverlap`
  (params (OtherActor :type "Actor Object Reference"))
  (bind _asbp_runner (cast `/Game/Runner/Blueprints/BP_Runner` OtherActor))
  (set `/Game/Runner/Blueprints/BP_Runner.Santé` (- (`/Game/Runner/Blueprints/BP_Runner.Santé` _asbp_runner) 20) _asbp_runner)
  ;[1 1 1] Appelle la fonction pour refresh les HP sur le dashboard
  (bind _returnvalue (`GameplayStatics.GetActorOfClass` "/Game/Runner/Blueprints/HUD/TextRender_Health.TextRender_Health_C"))
  (`/Game/Runner/Blueprints/HUD/TextRender_Health.RefreshHealthOnScreen` _returnvalue)
  (`GameplayStatics.PlaySound2D` "/Game/Runner/Sounds/Effects/Explosion_Cue.Explosion_Cue" 1.0 1.0 0.0 null null)
  (`/Game/Runner/Blueprints/BP_Runner.CameraShake` _asbp_runner)
  (`GameplayStatics.SpawnEmitterAtLocation` "/Game/StarterContent/Particles/P_Explosion.P_Explosion" (`self.K2_GetActorLocation`))
  (`self.K2_DestroyActor`))

(event `self.PawnSensing.OnSeePawn`
  (params (Pawn :type "Pawn Object Reference"))
  (cast `/Game/Runner/Blueprints/BP_Runner` Pawn)
  (`self.K2_SetActorRotation` (`KismetMathLibrary.FindLookAtRotation` (`self.K2_GetActorLocation`) (`self.K2_GetActorLocation` Pawn)))
  (`KismetSystemLibrary.Delay` 0.2)
  (`|SpawnActorFromClass` "/Game/Runner/Blueprints/Obstacles/BP_Bullets.BP_Bullets_C" (`SceneComponent.K2_GetComponentToWorld` (`self.Arrow`)) "Undefined" "MultiplyWithRoot" null null))

(event `self.ReceiveAnyDamage`
  (params (Damage :type "Float (single-precision)") (DamageType :type "DamageType Object Reference") (InstigatedBy :type "Controller Object Reference") (DamageCauser :type "Actor Object Reference"))
  (bind (_returnvalue_x _returnvalue_y _returnvalue_z) (`KismetMathLibrary.BreakVector` (`self.K2_GetActorLocation`)))
  ;[0.7396 0.3274 0.3274] Prendre damage de shotgun
  (if (> (`self.Health`) 0.0)
    (set `self.Health` (- (`self.Health`) Damage))
    (if (<= (`self.Health`) 0.0)
      (`GameplayStatics.SpawnEmitterAtLocation` "/Game/StarterContent/Particles/P_Explosion.P_Explosion" (`KismetMathLibrary.MakeVector` _returnvalue_x _returnvalue_y _returnvalue_z) (struct) (5.0 5.0 5.0))
      (`self.K2_DestroyActor`))))

(fn `UserConstructionScript`)
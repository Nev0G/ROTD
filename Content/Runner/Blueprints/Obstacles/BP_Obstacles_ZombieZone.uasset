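; Runner obstacle zone that spawns a random group of child actors at BeginPlay, presumably zombies given its name.
; It adds one to five unattached child actor components in a loop.
; Each takes the zone's height, rotation and scale, with X and Y randomized between the zone's own coordinate and a fixed absolute bound, rather than an offset around it.
; Tick is disabled and the construction script only calls its parent.
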(event `self.ReceiveBeginPlay`
  (bind _returnvalue (`self.GetTransform`))
  (`parent.ReceiveBeginPlay`)
  (bind _output_get (set `self.Last Index` (`KismetMathLibrary.RandomInteger` 5)))
  (for _ (range (+ _output_get 1))
    (`AddComponent|NODE_AddChildActorComponent-0` :`bManualAttachment` true :`RelativeTransform` (`KismetMathLibrary.MakeTransform` (`KismetMathLibrary.MakeVector` (`KismetMathLibrary.RandomFloatInRange` (.x (.location _returnvalue)) 20.0) (`KismetMathLibrary.RandomFloatInRange` (.y (.location _returnvalue)) 20.0) (.z (.location _returnvalue))) (.rotation _returnvalue) (.scale _returnvalue)))))

(fn `UserConstructionScript`
  (`parent.UserConstructionScript`))
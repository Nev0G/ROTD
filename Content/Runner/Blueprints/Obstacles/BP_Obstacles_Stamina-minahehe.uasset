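; Stamina pickup for the runner game that refills part of the player's Stamina on contact.
; When a BP_Runner overlaps it, a fixed amount is added to that runner's Stamina unless it equals exactly 100, with no clamping afterwards.
; Either way it plays the Ding sound and destroys itself.
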(event `self.ReceiveActorBeginOverlap`
  (params (OtherActor :type "Actor Object Reference"))
  (bind _asbp_runner (cast `/Game/Runner/Blueprints/BP_Runner` OtherActor))
  (if (== (`/Game/Runner/Blueprints/BP_Runner.Stamina` _asbp_runner) 100)
    ;[1 1 1] Si vie déja a 100 alors ntm
    (`GameplayStatics.PlaySound2D` "/Game/Runner/Sounds/Effects/Ding.Ding" 1.0 1.0 0.0 null null)
    (`self.K2_DestroyActor`)
    (else
      (set `/Game/Runner/Blueprints/BP_Runner.Stamina` (+ 10 (`/Game/Runner/Blueprints/BP_Runner.Stamina` _asbp_runner)) _asbp_runner)
      (`GameplayStatics.PlaySound2D` "/Game/Runner/Sounds/Effects/Ding.Ding" 1.0 1.0 0.0 null null)
      (`self.K2_DestroyActor`))))

(fn `UserConstructionScript`
  (`parent.UserConstructionScript`))
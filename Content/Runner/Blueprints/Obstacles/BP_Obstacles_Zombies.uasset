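; Zombie obstacle for the runner game that hurts the player's vehicle on contact and can be killed with weapon damage.
; On BeginPlay it picks a random skeletal mesh and animation.
; The first BP_Runner overlap triggers blood, health loss, a dashboard refresh and camera shake, with a random chance to attach a BP_ZombieCar to the runner.
; AnyDamage drains its health, then spawns gore and sound before destroying it.
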(event `self.ReceiveBeginPlay`
  (`parent.ReceiveBeginPlay`)
  (`self.RandomMesh`))

(event `self.ReceiveActorBeginOverlap`
  (params (OtherActor :type "Actor Object Reference"))
  (bind _asbp_runner (cast `/Game/Runner/Blueprints/BP_Runner` OtherActor))
  ;[1 0.04051 0.02061] Blood Splash
  (`/Engine/EditorBlueprintResources/StandardMacros.DoOnce` false
    (:`Completed`
      (`/Game/Runner/Blueprints/BP_Runner.BloodSplash` _asbp_runner)
      (if (`KismetMathLibrary.InRange_IntInt` (`KismetMathLibrary.RandomIntegerInRange` 0 100) 70 100)
        (set `/Game/Runner/Blueprints/BP_Runner.Santé` (- (`/Game/Runner/Blueprints/BP_Runner.Santé` _asbp_runner) 10) _asbp_runner)
        ;[1 0.7095 0.0916] Zombie monte sur voiture
        (bind _returnvalue (`|SpawnActorFromClass` "/Game/Runner/Blueprints/Obstacles/BP_ZombieCar.BP_ZombieCar_C" (`KismetMathLibrary.MakeTransform` (`KismetMathLibrary.MakeVector` -120.0 (`KismetMathLibrary.RandomFloatInRange` -150.0 150.0) 25.0) (struct :`Yaw` 90.0)) "AlwaysSpawn" "MultiplyWithRoot" null null))
        (`self.K2_AttachToActor` _returnvalue _asbp_runner "None" "KeepRelative" "KeepRelative" "KeepRelative" true)
        (else
          (set `/Game/Runner/Blueprints/BP_Runner.Santé` (- (`/Game/Runner/Blueprints/BP_Runner.Santé` _asbp_runner) 10) _asbp_runner)))
      ;[1 1 1] Appelle la fonction pour refresh les HP sur le dashboard
      (bind _returnvalue_2 (`GameplayStatics.GetActorOfClass` "/Game/Runner/Blueprints/HUD/TextRender_Health.TextRender_Health_C"))
      (`/Game/Runner/Blueprints/HUD/TextRender_Health.RefreshHealthOnScreen` _returnvalue_2)
      (`/Game/Runner/Blueprints/BP_Runner.CameraShake` _asbp_runner))))

(event `self.ReceiveAnyDamage`
  (params (Damage :type "Float (single-precision)") (DamageType :type "DamageType Object Reference") (InstigatedBy :type "Controller Object Reference") (DamageCauser :type "Actor Object Reference"))
  (bind (_returnvalue_x _returnvalue_y _returnvalue_z) (`KismetMathLibrary.BreakVector` (`self.K2_GetActorLocation`)))
  ;[0.7396 0.3274 0.3274] Prendre damage de shotgun
  (if (> (`self.Health`) 0.0)
    (set `self.Health` (- (`self.Health`) Damage))
    (if (<= (`self.Health`) 0.0)
      (`GameplayStatics.SpawnEmitterAtLocation` "/Game/Realistic_Starter_VFX_Pack_Vol2/Particles/Blood/P_Blood_Splat_Cone.P_Blood_Splat_Cone" (`KismetMathLibrary.MakeVector` _returnvalue_x _returnvalue_y _returnvalue_z) (struct) (5.0 5.0 5.0))
      (`GameplayStatics.PlaySoundAtLocation` "/Game/Runner/Sounds/Effects/ZombieProut.ZombieProut" (`KismetMathLibrary.MakeVector` _returnvalue_x _returnvalue_y _returnvalue_z) (struct) 1.0 1.0 0.0 null null null null)
      (`self.K2_DestroyActor`))))

(fn `RandomMesh`
  (`SkeletalMeshComponent.SetSkeletalMeshAsset` (`self.SkeletalMesh`) (`KismetArrayLibrary.Array_Random` (`self.MeshesList`)))
  (`SkeletalMeshComponent.SetAnimation` (`self.SkeletalMesh`) (`KismetArrayLibrary.Array_Random` (`self.AnimList`))))

(fn `UserConstructionScript`
  (`parent.UserConstructionScript`))
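; Runner obstacle that the player can only pass while sprinting, with a randomized look.
; On overlap, a sprinting BP_Runner has its capsule and box set to ignore the Destructible channel.
; Otherwise the capsule blocks that channel, the runner dies and the game pauses after a short delay.
; The construction script picks a random mesh from SprintMeshes and yaws it randomly to either side by a quarter turn.
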(event `self.ReceiveActorBeginOverlap`
  (params (OtherActor :type "Actor Object Reference"))
  (bind _asbp_runner (cast `/Game/Runner/Blueprints/BP_Runner` OtherActor))
  (if (`/Game/Runner/Blueprints/BP_Runner.isSprinting` _asbp_runner)
    (`PrimitiveComponent.SetCollisionResponseToChannel` (`Character.CapsuleComponent` _asbp_runner) "ECC_Destructible" "ECR_Ignore")
    (`PrimitiveComponent.SetCollisionResponseToChannel` (`/Game/Runner/Blueprints/BP_Runner.Box` _asbp_runner) "ECC_Destructible" "ECR_Ignore")
    (else
      (`PrimitiveComponent.SetCollisionResponseToChannel` (`Character.CapsuleComponent` _asbp_runner) "ECC_Destructible" "ECR_Block")
      (`/Game/Runner/Blueprints/BP_Runner.Death` _asbp_runner)
      (`KismetSystemLibrary.Delay` 1.0)
      (`GameplayStatics.SetGamePaused` true))))

(event `self.ReceiveTick`
  (params (DeltaSeconds :type "Float (single-precision)"))
  (`parent.ReceiveTick` DeltaSeconds))

(fn `UserConstructionScript`
  (bind _staticmesh (`self.StaticMesh`))
  ;[1 0.1039 0] Random Mesh
  (`parent.UserConstructionScript`)
  (`StaticMeshComponent.SetStaticMesh` _staticmesh (`|GetArrayItem` (`self.SprintMeshes`) (`KismetMathLibrary.RandomIntegerInRange` 0 (- (`KismetArrayLibrary.Array_Length` (`self.SprintMeshes`)) 1))))
  ;[0.922 0 1] Random Rotation
  (set `self.Rotation` (`KismetMathLibrary.RandomIntegerInRange` 0 1))
  (if (== (`self.Rotation`) 0)
    (set `self.Rotation` -90)
    (else
      (set `self.Rotation` 90)))
  (`SceneComponent.K2_SetRelativeRotation` _staticmesh (`KismetMathLibrary.MakeRotator` 0.0 0.0 (`KismetMathLibrary.Conv_IntToDouble` (`self.Rotation`))) false false))
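; Shotgun ammo pickup for the runner game, consumed when the BP_Runner character overlaps it.
; It adds a fixed amount to the runner's ShottyAmmo, clamps it to ShottyMaxAmmo, then refreshes the TextRender_Bullets display found via GetActorOfClass.
; If ammo is already full, it skips the refill and refresh, but still plays the Ding sound and destroys itself.
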(event `self.ReceiveActorBeginOverlap`
  (params (OtherActor :type "Actor Object Reference"))
  (bind _asbp_runner (cast `/Game/Runner/Blueprints/BP_Runner` OtherActor))
  (if (== (`/Game/Runner/Blueprints/BP_Runner.ShottyAmmo` _asbp_runner) (`/Game/Runner/Blueprints/BP_Runner.ShottyMaxAmmo` _asbp_runner))
    (`GameplayStatics.PlaySound2D` "/Game/Runner/Sounds/Effects/Ding.Ding" 1.0 1.0 0.0 null null)
    (`self.K2_DestroyActor`)
    (else
      (set `/Game/Runner/Blueprints/BP_Runner.ShottyAmmo` (+ (`/Game/Runner/Blueprints/BP_Runner.ShottyAmmo` _asbp_runner) 3) _asbp_runner)
      (bind _shottymaxammo (`/Game/Runner/Blueprints/BP_Runner.ShottyMaxAmmo` _asbp_runner))
      (if (> (`/Game/Runner/Blueprints/BP_Runner.ShottyAmmo` _asbp_runner) _shottymaxammo)
        (set `/Game/Runner/Blueprints/BP_Runner.ShottyAmmo` _shottymaxammo _asbp_runner))
      (bind _returnvalue (`GameplayStatics.GetActorOfClass` "/Game/Runner/Blueprints/HUD/TextRender_Bullets.TextRender_Bullets_C"))
      (`/Game/Runner/Blueprints/HUD/TextRender_Bullets.RefreshBulletsOnScreen` _returnvalue)
      (`GameplayStatics.PlaySound2D` "/Game/Runner/Sounds/Effects/Ding.Ding" 1.0 1.0 0.0 null null)
      (`self.K2_DestroyActor`))))

(fn `UserConstructionScript`
  (`parent.UserConstructionScript`))
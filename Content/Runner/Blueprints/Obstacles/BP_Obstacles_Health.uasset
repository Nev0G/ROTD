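; Health pickup for the runner game that heals BP_Runner on overlap and then destroys itself.
; It adds a fixed amount to the runner's Santé, clamped to MaxHealth, finds TextRender_Health with GetActorOfClass to refresh the on-screen value, and plays a pickup sound.
; At full health it skips healing and the refresh, plays a ding and is still consumed.
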(event `self.ReceiveActorBeginOverlap`
  (params (OtherActor :type "Actor Object Reference"))
  (bind _asbp_runner (cast `/Game/Runner/Blueprints/BP_Runner` OtherActor))
  (if (== (`/Game/Runner/Blueprints/BP_Runner.Santé` _asbp_runner) (`/Game/Runner/Blueprints/BP_Runner.MaxHealth` _asbp_runner))
    ;[1 1 1] Si Stamina deja a 100 alors ntm
    (`GameplayStatics.PlaySound2D` "/Game/Runner/Sounds/Effects/Ding.Ding" 1.0 1.0 0.0 null null)
    (`self.K2_DestroyActor`)
    (else
      (set `/Game/Runner/Blueprints/BP_Runner.Santé` (+ 10 (`/Game/Runner/Blueprints/BP_Runner.Santé` _asbp_runner)) _asbp_runner)
      (bind _maxhealth (`/Game/Runner/Blueprints/BP_Runner.MaxHealth` _asbp_runner))
      (if (> (`/Game/Runner/Blueprints/BP_Runner.Santé` _asbp_runner) _maxhealth)
        (set `/Game/Runner/Blueprints/BP_Runner.Santé` _maxhealth _asbp_runner))
      ;[1 1 1] Appelle la fonction pour refresh les HP sur le dashboard
      (bind _returnvalue (`GameplayStatics.GetActorOfClass` "/Game/Runner/Blueprints/HUD/TextRender_Health.TextRender_Health_C"))
      (`/Game/Runner/Blueprints/HUD/TextRender_Health.RefreshHealthOnScreen` _returnvalue)
      (`GameplayStatics.PlaySound2D` "/Game/Runner/Sounds/Effects/pickup.pickup" 1.0 1.0 0.0 null null)
      (`self.K2_DestroyActor`))))

(event `SetMaxHealth_1`)

(fn `UserConstructionScript`
  (`parent.UserConstructionScript`))
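; BP_Obstacles_Bombe is a bomb obstacle for the runner game that damages the player on contact.
; On actor overlap it casts the other actor to BP_Runner and subtracts a fixed amount from its Santé (health).
; It then plays a 2D explosion sound, spawns an explosion particle emitter and destroys itself, while any non-runner overlap is ignored.
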(event `self.ReceiveActorBeginOverlap`
  (params (OtherActor :type "Actor Object Reference"))
  (bind _asbp_runner (cast `/Game/Runner/Blueprints/BP_Runner` OtherActor))
  (set `/Game/Runner/Blueprints/BP_Runner.Santé` (- (`/Game/Runner/Blueprints/BP_Runner.Santé` _asbp_runner) 10) _asbp_runner)
  (`GameplayStatics.PlaySound2D` "/Game/Runner/Sounds/Effects/Explosion_Cue.Explosion_Cue" 1.0 1.0 0.0 null null)
  (`GameplayStatics.SpawnEmitterAtLocation` "/Game/StarterContent/Particles/P_Explosion.P_Explosion")
  (`self.K2_DestroyActor`))

(fn `UserConstructionScript`
  (`parent.UserConstructionScript`))
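; BP_Bullets is a runner-game obstacle that damages the player on contact.
; On overlap with BP_Runner, it subtracts a fixed amount from Santé (health) and has the TextRender_Health actor, found by class lookup, refresh the on-screen display.
; It then plays a 2D laser sound, triggers the runner's camera shake, spawns an explosion at the runner's location and destroys itself.
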(event `self.ReceiveActorBeginOverlap`
  (params (OtherActor :type "Actor Object Reference"))
  (bind _asbp_runner (cast `/Game/Runner/Blueprints/BP_Runner` OtherActor))
  (set `/Game/Runner/Blueprints/BP_Runner.Santé` (- (`/Game/Runner/Blueprints/BP_Runner.Santé` _asbp_runner) 10) _asbp_runner)
  ;[1 1 1] Appelle la fonction pour refresh les HP sur le dashboard
  (bind _returnvalue (`GameplayStatics.GetActorOfClass` "/Game/Runner/Blueprints/HUD/TextRender_Health.TextRender_Health_C"))
  (`/Game/Runner/Blueprints/HUD/TextRender_Health.RefreshHealthOnScreen` _returnvalue)
  (`GameplayStatics.PlaySound2D` "/Engine/VREditor/Sounds/UI/Laser_Push.Laser_Push" 1.0 1.0 0.0 null null)
  (`/Game/Runner/Blueprints/BP_Runner.CameraShake` _asbp_runner)
  (`GameplayStatics.SpawnEmitterAtLocation` "/Game/StarterContent/Particles/P_Explosion.P_Explosion" (`self.K2_GetActorLocation` _asbp_runner))
  (`self.K2_DestroyActor`))

(fn `UserConstructionScript`)
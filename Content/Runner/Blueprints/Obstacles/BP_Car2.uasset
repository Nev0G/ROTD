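; BP_Car2 is a moving car obstacle for the runner game that kills BP_Runner on contact.
; When the runner enters BoxOverlap, a sound plays and a timeline slides the mesh along world X toward the Arrow, lerping from its current position each update.
; The actor destroys itself five seconds after the move ends.
; Overlapping the CAR component calls the runner's Death, then pauses the game after a one-second delay.
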(event `self.CAR.OnComponentBeginOverlap`
  (params (OverlappedComponent :type "PrimitiveComponent Object Reference") (OtherActor :type "Actor Object Reference") (OtherComp :type "PrimitiveComponent Object Reference") (OtherBodyIndex :type Integer) (bFromSweep :type Boolean) (SweepResult :type "HitResult Structure (by ref)"))
  (bind _asbp_runner (cast `/Game/Runner/Blueprints/BP_Runner` OtherActor))
  (`/Game/Runner/Blueprints/BP_Runner.Death` _asbp_runner)
  (`KismetSystemLibrary.Delay` 1.0)
  (`GameplayStatics.SetGamePaused` true))

(event `self.Box Overlap.OnComponentBeginOverlap`
  (params (OverlappedComponent :type "PrimitiveComponent Object Reference") (OtherActor :type "Actor Object Reference") (OtherComp :type "PrimitiveComponent Object Reference") (OtherBodyIndex :type Integer) (bFromSweep :type Boolean) (SweepResult :type "HitResult Structure (by ref)"))
  (bind _staticmesh (`self.StaticMesh`))
  (cast `/Game/Runner/Blueprints/BP_Runner` OtherActor)
  (`GameplayStatics.SpawnSoundAttached` "/Game/StarterContent/Audio/Collapse_Cue.Collapse_Cue" (`self.StaticMesh`) "None" (0.0 0.0 0.0) (struct) "KeepRelativeOffset" false 1.0 1.0 0.0 null null)
  (bind (_direction _move_obstacle) (`Timeline|Chronologie` :!via `PlayFromStart`)
    (:`Update`
      (`SceneComponent.K2_SetWorldLocation` _staticmesh (`KismetMathLibrary.MakeVector` (`KismetMathLibrary.Lerp` (.x (`SceneComponent.K2_GetComponentLocation` _staticmesh)) (.x (`SceneComponent.K2_GetComponentLocation` (`self.Arrow`))) _move_obstacle) (.y (`SceneComponent.K2_GetComponentLocation` _staticmesh)) (.z (`SceneComponent.K2_GetComponentLocation` _staticmesh))) false false))
    (:`Finished`
      (`KismetSystemLibrary.Delay` 5.0)
      (`self.K2_DestroyActor`))))

(fn `UserConstructionScript`)
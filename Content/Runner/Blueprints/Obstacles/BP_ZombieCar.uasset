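; BP_ZombieCar is a zombie obstacle that drains the runner's health while overlapping it and can be destroyed by damage.
; Overlap start sets the Exist flag, plays a growl, then loops on a one-second Delay, decrementing BP_Runner's Santé and refreshing the TextRender_Health display.
; Overlap end clears the flag to stop the loop.
; AnyDamage, noted as shotgun damage, lowers the zombie's Health and destroys it at zero.
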(event `self.ReceiveBeginPlay`)

(event `self.ReceiveActorBeginOverlap`
  (params (OtherActor :type "Actor Object Reference"))
  (if (not (`self.Exist?`))
    (set `self.Exist?` true)
    (`GameplayStatics.PlaySoundAtLocation` "/Game/Runner/Sounds/ZombieGrowl.ZombieGrowl" (`self.GetActorEyesViewPoint`) (struct) 1.0 1.0 0.0 null null null null)
    (bind _asbp_runner (cast `/Game/Runner/Blueprints/BP_Runner` OtherActor))
    (if (`self.Exist?`) :!label _label
      (`KismetSystemLibrary.PrintString` "ZOMBIE EXISTE")
      (set `/Game/Runner/Blueprints/BP_Runner.Santé` (- (`/Game/Runner/Blueprints/BP_Runner.Santé` _asbp_runner) 1) _asbp_runner)
      ;[1 1 1] Appelle la fonction pour refresh les HP sur le dashboard
      (bind _returnvalue (`GameplayStatics.GetActorOfClass` "/Game/Runner/Blueprints/HUD/TextRender_Health.TextRender_Health_C"))
      (`/Game/Runner/Blueprints/HUD/TextRender_Health.RefreshHealthOnScreen` _returnvalue)
      (`KismetSystemLibrary.Delay` 1.0)
      (goto _label))))

(event `self.ReceiveActorEndOverlap`
  (params (OtherActor :type "Actor Object Reference"))
  (set `self.Exist?` false))

(event `self.ReceiveAnyDamage`
  (params (Damage :type "Float (single-precision)") (DamageType :type "DamageType Object Reference") (InstigatedBy :type "Controller Object Reference") (DamageCauser :type "Actor Object Reference"))
  ;[0.7396 0.3274 0.3274] Prendre damage de shotgun
  (if (> (`self.Health`) 0.0)
    (set `self.Health` (- (`self.Health`) Damage))
    (if (<= (`self.Health`) 0.0)
      (`self.K2_DestroyActor`))))

(fn `UserConstructionScript`)
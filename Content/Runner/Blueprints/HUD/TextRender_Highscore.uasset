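; World-space TextRender actor that displays the runner's high score in the Runner game.
; RefreshScoreOnScreen finds all BP_Runner actors, takes the first one's Highscore and writes it to the text component as a whole number.
; The refresh runs on BeginPlay and whenever the GetSpeed_1 event fires, with no per-frame update.
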(event `GetSpeed_1`
  (`self.RefreshScoreOnScreen`))

(event `self.ReceiveBeginPlay`
  (`self.RefreshScoreOnScreen`))

(fn `RefreshScoreOnScreen`
  (bind _outactors (`GameplayStatics.GetAllActorsOfClass` "/Game/Runner/Blueprints/BP_Runner.BP_Runner_C"))
  (`TextRenderComponent.K2_SetText` (`self.TextRender`) (`KismetTextLibrary.Conv_Int64ToText` (`KismetMathLibrary.Conv_IntToInt64` (`/Game/Runner/Blueprints/BP_Runner.Highscore` (`|GetArrayItem` _outactors))) false false)))

(fn `UserConstructionScript`)
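; A text render actor that displays the runner's current speed.
; RefreshSpeedOnScreen takes the first BP_Runner found in the world, truncates its velocity magnitude to an integer, divides by ten and writes the result as text.
; The refresh runs once at BeginPlay and again whenever the GetSpeed event is called, with no per-frame update in this Blueprint.
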(event `/Game/Runner/Blueprints/Interfaces/GetSpeedInterface.GetSpeed`
  (`self.RefreshSpeedOnScreen`))

(event `self.ReceiveBeginPlay`
  (`self.RefreshSpeedOnScreen`))

(fn `RefreshSpeedOnScreen`
  (bind _outactors (`GameplayStatics.GetAllActorsOfClass` "/Game/Runner/Blueprints/BP_Runner.BP_Runner_C"))
  (`TextRenderComponent.K2_SetText` (`self.TextRender`) (`KismetTextLibrary.Conv_Int64ToText` (/ (`KismetMathLibrary.Conv_DoubleToInt64` (`KismetMathLibrary.VSize` (`self.GetVelocity` (`|GetArrayItem` _outactors)))) 10))))

(fn `UserConstructionScript`)